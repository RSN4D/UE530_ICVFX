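; BP_LX_Control is a control actor that generates and randomizes point lights in the level.
; SpawnLights destroys every PointLight, then spawns a configurable number attached to the first BP_LX_Root.
; The construction script runs Update, which gives every PointLight a random relative position and candela intensity within set ranges, Movable mobility and a fixed attenuation radius.
; Both functions affect all PointLights in the level, and the event graph is unused.
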(event EventBeginPlay)

(event Collision|EventActorBeginOverlap
  (params (OtherActor :type Actor%20Object%20Reference)))

(event EventTick
  (params (DeltaSeconds :type Float%20%28single-precision%29)))

(fn ConstructionScript
  (CallFunction|Update))

(fn Update
  (bind _outactors (Actor|GetAllActorsOfClass "/Script/Engine.PointLight"))
  (bind _output_get (Variables|Default|SetOut%20Actors _outactors))
  (for _array_element _output_get
    (Transformation|SetActorRelativeLocation _array_element (Math|Vector|MakeVector (Math|Random|RandomFloatinRange (Variables|LX|GetMinX) (Variables|LX|GetMaxX)) (Math|Random|RandomFloatinRange (Variables|LX|GetMinY) (Variables|LX|GetMaxY)) (Math|Random|RandomFloatinRange (Variables|LX|GetMinZ) (Variables|LX|GetMaxZ))))
    (Transformation|SetMobility (Variables|/Script/Engine.Light|GetLightComponent _array_element) "Movable")
    (Class|LocalLightComponent|SetIntensityUnits (Variables|/Script/Engine.PointLight|GetPointLightComponent _array_element) "Candelas")
    (Rendering|Components|Light|SetIntensity (Variables|/Script/Engine.PointLight|GetPointLightComponent _array_element) (Math|Random|RandomFloatinRange (Variables|LX|GetMinLX) (Variables|LX|GetMaxLX)))
    (Rendering|Lighting|SetAttenuationRadius (Variables|/Script/Engine.PointLight|GetPointLightComponent _array_element) 5e+03)))

(fn SpawnLights
  (bind _actorstospawn (Variables|Default|GetActorsToSpawn))
  (bind _outactors (Actor|GetAllActorsOfClass "/Script/Engine.PointLight"))
  (for _array_element _outactors
    (Actor|DestroyActor _array_element))
  (Utilities|Array|Resize _actorstospawn (Variables|Amount|GetLX%20Amount))
  (for _array_element_2 _actorstospawn
    (bind _outactors_2 (Actor|GetAllActorsOfClass "/Game/C_LX/BP_LX_Root.BP_LX_Root_C"))
    (bind _returnvalue (Game|SpawnActorfromClass "/Script/Engine.PointLight" (Variables|Default|GetSpawn%20Transform) "Undefined" "MultiplyWithRoot" 0 0))
    (Transformation|AttachActorToActor _returnvalue (Utilities|Array|Get(acopy) _outactors_2) "None" "KeepRelative" "KeepRelative" "KeepRelative" true)))